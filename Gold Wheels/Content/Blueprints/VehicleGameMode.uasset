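; Game mode for a vehicle game that shows the HUD and ends the match on a score target.
; BeginPlay adds the HUD widget, and every Tick runs CheckScore, which opens EndMenu once the player pawn's Score reaches ScoreToWin.
; Tick also drives a seconds timer through a one-second Delay.
; TimeSec wraps after 59, but TimeMin is assigned to itself, so minutes never advance.
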(event EventTick
  (params (DeltaSeconds :type Float%20%28single-precision%29))
  (CallFunction|CheckScore)
  (Utilities|FlowControl|Delay 1.0)
  (Variables|Default|SetTimeSec (+ (Variables|Default|GetTimeSec) 1))
  (if (> (Variables|Default|GetTimeSec) 59)
    (Variables|Default|SetTimeMin (Variables|Default|GetTimeMin))
    (Variables|Default|SetTimeSec 0)))

(event EventBeginPlay
  (bind _returnvalue (UserInterface|CreateWidget "/Game/Blueprints/HUD.HUD_C"))
  (UserInterface|Viewport|AddtoViewport _returnvalue 0))

(fn ConstructionScript)

(fn CheckScore
  (bind _asmy_vehicle_template_pawn (Utilities|Casting|CastToMyVehicleTemplatePawn (Game|Player|GetPlayerPawn 0)))
  (if (>= (Variables|/Game/Blueprints/MyVehicleTemplatePawn.MyVehicleTemplatePawn_C|GetScore _asmy_vehicle_template_pawn) (Variables|Default|GetScoreToWin))
    (Game|OpenLevel(byName) "EndMenu")))